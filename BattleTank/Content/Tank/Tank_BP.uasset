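; Player-drivable tank pawn that hands driving, aiming and firing to its TankMovement and TankAiming components.
; On BeginPlay it wires the barrel, turret and both tracks into those components and links the health bar widget to itself.
; Move and turn axes feed TankMovement intents, while aim axes rotate the azimuth gimbal and spring arm, scaled by delta time.
; The fire action calls TankAiming to shoot.
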(event `self.ReceiveBeginPlay`
  (`TankAimingComponent.Initialize` (`self.TankAiming`) (`self.Barrel`) (`self.Turret`))
  (`TankMovementComponent.Initialize` (`self.TankMovement`) (`self.LeftTrack`) (`self.RightTrack`))
  ;[1 1 1] Double-click to see inside
  (`self.InitializeHealthBarWidget`))

(event `InputAxis|AimAzimuth`
  (params (AxisValue :type "Float (single-precision)"))
  ;[1 1 1] Baliistics Input Binding
  (`SceneComponent.K2_AddLocalRotation` (`self.Azimuth Gimbal`) (`KismetMathLibrary.MakeRotator` 0.0 0.0 (* AxisValue (`GameplayStatics.GetWorldDeltaSeconds`) 100.0)) false false))

(event `InputAxis|Move Forward`
  (params (AxisValue :type "Float (single-precision)"))
  ;[1 1 1] Movement Input Bindings
  (`TankMovementComponent.IntendMoveForward` (`self.TankMovement`) AxisValue))

(event `InputAxis|Turn Right`
  (params (AxisValue :type "Float (single-precision)"))
  ;[1 1 1] Movement Input Bindings
  (`TankMovementComponent.IntendTurnRight` (`self.TankMovement`) AxisValue))

(event `InputAxis|AimElevation`
  (params (AxisValue :type "Float (single-precision)"))
  ;[1 1 1] Baliistics Input Binding
  (`SceneComponent.K2_AddLocalRotation` (`self.SpringArm`) (`KismetMathLibrary.MakeRotator` 0.0 (* AxisValue (`GameplayStatics.GetWorldDeltaSeconds`) 100.0)) false false))

(event `InputAction|Fire`
  (params (Key :type "Key Structure"))
  ;[1 1 1] Baliistics Input Binding
  (:`Pressed`
    (`TankAimingComponent.Fire` (`self.TankAiming`))))

(fn `InitializeHealthBarWidget`
  (bind _ashealth_bar_bp (cast `/Game/UI/HealthBar_BP` (`WidgetComponent.GetUserWidgetObject` (`self.HealthBar`))))
  (set `/Game/UI/HealthBar_BP.MyTank` self _ashealth_bar_bp)
  (return))

(fn `UserConstructionScript`)